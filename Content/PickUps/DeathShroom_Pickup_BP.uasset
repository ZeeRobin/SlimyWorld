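; DeathShroom_Pickup_BP is a deadly mushroom pickup that ends the game when the SlimeCharacter overlaps it.
; It destroys the character, then after a short delay plays a scream at its mesh and destroys itself.
; It then shows a GameOver2 widget, creating it if needed, and switches to UI-only input with a visible cursor.
; A final delayed pause is scheduled after the pickup's own DestroyActor call.
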(event EventBeginPlay)

(event Collision|EventActorBeginOverlap
  (params (OtherActor :type Actor%20Object%20Reference))
  (bind _asslime_character (Utilities|Casting|CastToSlimeCharacter OtherActor))
  (Actor|DestroyActor _asslime_character)
  (Utilities|FlowControl|Delay 0.5)
  (Audio|PlaySoundatLocation "/Game/Sounds/Roblox_Screaming.Roblox_Screaming" (Transformation|GetWorldLocation (Variables|Default|GetStaticMesh)) "0, 0, 0" 1.0 1.0 0.0 0 0 0)
  (Actor|DestroyActor)
  (Utilities|IsValid (Variables|Default|GetGameOver)
    (:Is%20Valid
      _)
    (:Is%20Not%20Valid
      (bind _returnvalue (UserInterface|CreateWidget "/Game/Widgets/GameOver2.GameOver2_C" (Game|GetPlayerController 0)))
      (Variables|Default|SetGameOver _returnvalue)))
  (UserInterface|Viewport|AddtoViewport (Variables|Default|GetGameOver) 0)
  (Input|SetInputModeUIOnly (Game|GetPlayerController 0) (Variables|Default|GetGameOver) "DoNotLock")
  (Variables|/Script/Engine.PlayerController|SetbShowMouseCursor (Game|GetPlayerController 0) true)
  (Utilities|FlowControl|Delay 0.8)
  (Game|SetGamePaused true))

(event EventTick
  (params (DeltaSeconds :type Float%20%28single-precision%29)))

(fn ConstructionScript)